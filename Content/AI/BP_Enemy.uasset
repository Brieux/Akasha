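; Flying elemental enemy that chases the first player pawn it senses, self-destructing on contact, out of height bounds or after a timeout.
; Construction draws its weakness from a phase-based pool, setting mesh, animation, resistance and Niagara colour.
; GetHit kills on weakness, ignores resistance and otherwise drains PV, except in wave two where any hit kills.
; Kills charge the player's ultimate and can advance waves; any destruction calls PlayerPawn's LosePV.
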(event OnSeePawn(PawnSensing)
  (params (Pawn :type Pawn%20Object%20Reference))
  (Variables|Default|GetTarget
    (:then)
    (:else
      (bind _asplayer_pawn (Utilities|Casting|CastToPlayerPawn Pawn)
        (:then
          (Variables|Default|SetTarget _asplayer_pawn))
        (:CastFailed
          (bind _asbp_first_person_character (Utilities|Casting|CastToBP_FirstPersonCharacter Pawn))
          (Variables|Default|SetTarget _asbp_first_person_character))))))

(event OnComponentBeginOverlap(CapsuleComponent)
  (params (OverlappedComponent :type Primitive%20Component%20Object%20Reference) (OtherActor :type Actor%20Object%20Reference) (OtherComp :type Primitive%20Component%20Object%20Reference) (OtherBodyIndex :type Integer) (bFromSweep :type Boolean) (SweepResult :type Hit%20Result%20Structure%20%28by%20ref%29))
  (bind _returnvalue (Game|Player|GetPlayerPawn 0))
  (if (== OtherActor (Variables|Default|GetTarget))
    (Class|BPIGameModeMP|RemoveOneEnemy(Message) (Game|GetGameMode))
    (bind _asplayer_pawn (Utilities|Casting|CastToPlayerPawn _returnvalue)
      (:then
        (Default|LosePV _asplayer_pawn))
      (:CastFailed
        (Utilities|Casting|CastToBP_FirstPersonCharacter _returnvalue)
        (Development|PrintString "Loose pv fps")))
    (Actor|DestroyActor)
    (elif (Variables|Default|GetStrafeDirection)
      (Pawn|Input|AddMovementInput "0.000000,10.000000,0.000000" 0.1 false)
      (else
        (Pawn|Input|AddMovementInput "0.000000,-10.000000,0.000000" 0.1 false)))))

(event Custom|InactiveDestroy
  (Class|BPIGameModeMP|RemoveOneEnemy(Message) (Game|GetGameMode))
  (Actor|DestroyActor))

(event EventBeginPlay
  (CallFunction|SetFlySpeed (Variables|Default|GetMax%20Fly%20Speed))
  (Utilities|Time|SetTimerbyEvent (delegate Custom|InactiveDestroy) 6e+01))

(event EventDestroyed
  (bind _asplayer_pawn (Utilities|Casting|CastToPlayerPawn (Game|Player|GetPlayerPawn 0)))
  (Default|LosePV _asplayer_pawn))

(event EventTick
  (params (DeltaSeconds :type Float%20%28single-precision%29))
  (bind _returnvalue (Transformation|GetActorLocation))
  (bind _returnvalue_2 (Transformation|GetActorLocation))
  (bind _target (Variables|Default|GetTarget))
  (bind _returnvalue_3 (Transformation|GetActorLocation _target))
  (if (or (< (.z _returnvalue) -4e+02) (> (.z _returnvalue) 4e+02))
    (Class|BPIGameModeMP|RemoveOneEnemy(Message) (Game|GetGameMode))
    (Actor|DestroyActor)
    (else
      (bind _target_2 (Variables|Default|GetTarget)
        (:then
          (if (> (Transformation|GetDistanceTo _target_2) (Variables|Default|GetDistanceToStop))
            (Pawn|Input|AddMovementInput (Math|Rotator|GetRotationXVector (Math|Rotator|FindLookatRotation (Transformation|GetActorLocation) (Transformation|GetActorLocation _target_2))) 1.0 false)
            (Transformation|SetActorRotation (Math|Rotator|FindLookatRotation (Transformation|GetActorLocation) (Transformation|GetActorLocation _target_2)))
            (if (> (.z _returnvalue_2) (.z _returnvalue_3))
              (Pawn|Input|AddMovementInput "0.000000,0.000000,1.000000" 0.1 false)
              (elif (not (== (.z _returnvalue_2) (.z _returnvalue_3)))
                (Pawn|Input|AddMovementInput "0.000000,0.000000,-1.000000" 0.1 false)))))
        (:else)))))

(fn ConstructionScript
  (bind _mesh (Variables|Character|GetMesh))
  (bind _actualphase (Class|BPIGameModeMP|GetActualPhase(Message) (Game|GetGameMode)))
  (Variables|Default|SetNumeroPhase _actualphase)
  (Utilities|FlowControl|Sequence
    (:then_0
      (if (== (Math|Random|RandomIntegerinRange 0 1) 1)
        (Variables|Default|SetStrafeDirection true)
        (else
          (Variables|Default|SetStrafeDirection false))))
    (:then_1
      (bind _output_get (Variables|Default|SetElementWeak (Utilities|Select :Index (.OutItem (Utilities|Array|Random (Utilities|Select :Index (Variables|Default|GetNumeroPhase) :Option%200 (Utilities|Array|MakeArray 2 4) :Option%201 (Utilities|Array|MakeArray 2 4 1) :Option%202 (Utilities|Array|MakeArray 2 4 1 3)))) :Option%200 "NewEnumerator0" :Option%201 "NewEnumerator3" :Option%202 "NewEnumerator4" :Option%203 "NewEnumerator2" :Option%204 "NewEnumerator1")))
      (Components|SkeletalMesh|SetSkeletalMeshAsset _mesh (Utilities|Select :Index _output_get :NewEnumerator0 "/Game/Characters/Mannequin_UE4/Meshes/SK_Mannequin.SK_Mannequin" :NewEnumerator1 "/Game/Esprits/Fire/FuegoRigSmooth.FuegoRigSmooth" :NewEnumerator2 "/Game/Esprits/Earth/GeoRigSmooth.GeoRigSmooth" :NewEnumerator3 "/Game/Esprits/Water/Spirit_Rig.Spirit_Rig" :NewEnumerator4 "/Game/Esprits/Eol/EolRig.EolRig"))
      (Components|Animation|SetAnimationMode _mesh "AnimationBlueprint")
      (Class|SkeletalMeshComponent|SetAnimClass _mesh (Utilities|Select :Index _output_get :NewEnumerator0 0 :NewEnumerator1 "/Game/Esprits/Fire/ABP_Fuego.ABP_Fuego_C" :NewEnumerator2 "/Game/Esprits/Earth/ABP_Geo.ABP_Geo_C" :NewEnumerator3 "/Game/Esprits/Water/ABP_EAU.ABP_EAU_C" :NewEnumerator4 "/Game/Esprits/Eol/ABP_Eol.ABP_Eol_C")))
    (:then_2
      (Transformation|SetActorRotation (Math|Rotator|FindLookatRotation (Transformation|GetActorLocation) (Math|Vector|MakeVector 0.0 0.0 0.0))))
    (:then_3
      (bind _output_get_2 (Variables|Default|SetResistElement (Utilities|Select :Index (Variables|Default|GetElementWeak) :NewEnumerator0 "NewEnumerator0" :NewEnumerator1 "NewEnumerator4" :NewEnumerator2 "NewEnumerator3" :NewEnumerator3 "NewEnumerator1" :NewEnumerator4 "NewEnumerator2")))
      (Niagara|SetNiagaraVariable(LinearColor) (Variables|Default|GetNiagara) "UseColor" (Utilities|Select :Index _output_get_2 :NewEnumerator0 "" :NewEnumerator1 (Variables|Default|GetWater) :NewEnumerator2 (Variables|Default|GetWind) :NewEnumerator3 (Variables|Default|GetEarth) :NewEnumerator4 (Variables|Default|GetFire))))))

(fn GetHit
  (params (Element :type Byte))
  (bind _returnvalue (Game|GetGameMode))
  (bind _returnvalue_2 (Game|Player|GetPlayerPawn 0))
  (bind _returnvalue_3 (Game|GetGameMode))
  (bind _wavenb (Class|BPIGameModeMP|GetWaveNb(Message) (Game|GetGameMode)))
  (if (== _wavenb 2)
    (bind _asplayer_pawn (Utilities|Casting|CastToPlayerPawn _returnvalue_2 :!label _label)
      (:then
        (bind _output_get (Variables|/Game/VRTemplate/Blueprints/PlayerPawn.PlayerPawn_C|SetUltGauge _asplayer_pawn (Math|Float|Clamp(Float) (+ (Variables|/Game/VRTemplate/Blueprints/PlayerPawn.PlayerPawn_C|GetUltGauge _asplayer_pawn) (Variables|Default|GetIncrementUlti)))))
        (bind _wavenb_2 (Class|BPIGameModeMP|GetWaveNb(Message) _returnvalue))
        (if (and (== _output_get 1.0) (== _wavenb_2 1))
          (Class|BPIGameModeMP|NextWave(Message) _returnvalue_3 :!label _label_2)
          (Default|CycleMusic _asplayer_pawn)
          (Utilities|FlowControl|Sequence
            (:then_0
              (Utilities|FlowControl|FlipFlop
                (:A
                  (Variables|Default|SetIncrementUlti 0.05))
                (:B
                  (Variables|Default|SetIncrementUlti 0.008))))
            (:then_1
              (Class|BPIGameModeMP|RemoveOneEnemy(Message) _returnvalue_3 :!label _label_3)
              (Class|BPIGameModeMP|RemoveOneBossNbEnemies(Message) _returnvalue_3)
              (Actor|DestroyActor)))
          (else
            (goto _label_3))))
      (:CastFailed
        (bind _asbp_first_person_character (Utilities|Casting|CastToBP_FirstPersonCharacter _returnvalue_2))
        (bind _output_get_2 (Variables|/Game/FirstPerson/Blueprints/BP_FirstPersonCharacter.BP_FirstPersonCharacter_C|SetUltiGauge _asbp_first_person_character (Math|Float|Clamp(Float) (+ (Variables|/Game/FirstPerson/Blueprints/BP_FirstPersonCharacter.BP_FirstPersonCharacter_C|GetUltiGauge _asbp_first_person_character) (Variables|Default|GetIncrementUlti)))))
        (bind _wavenb_3 (Class|BPIGameModeMP|GetWaveNb(Message) _returnvalue))
        (if (and (== _wavenb_3 1) (== _output_get_2 1.0))
          (goto _label_2)
          (else
            (goto _label_3)))))
    (elif (== Element (Math|Conversions|ToInteger(Byte) (Variables|Default|GetElementWeak)))
      (goto _label)
      (elif (not (== Element (Math|Conversions|ToInteger(Byte) (Variables|Default|GetResistElement))))
        (bind _output_get_3 (Variables|Default|SetPV (- (Variables|Default|GetPV) 1)))
        (if (== _output_get_3 0)
          (goto _label))))))

(fn SetFlySpeed
  (params (Speed :type Float%20%28double-precision%29))
  (Variables|/Script/Engine.CharacterMovementComponent|SetMaxFlySpeed (Variables|Character|GetCharacterMovement) Speed))