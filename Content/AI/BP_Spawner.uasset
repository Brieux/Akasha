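; BP_Spawner is an enemy spawner that creates BP_Enemy AI inside a box zone, scaled by SpawnScale at BeginPlay.
; It registers with the GameMode through message calls, and SpawnOneEnemy asks it for permission, then reports each spawn back.
; A loop rerolls a random point until it is at least MinRange from the player, but the spawn uses a fresh random point, so that check is not applied.
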(event Custom|SpawnOneEnemy
  (bind _enemiesspawnzone (Variables|Default|GetEnemiesSpawnZone))
  (bind _returnvalue (Components|Box|GetScaledBoxExtent _enemiesspawnzone))
  (bind _returnvalue_2 (Transformation|GetWorldLocation _enemiesspawnzone))
  (bind _returnvalue_3 (Math|Random|RandomPointinBoundingBox _returnvalue_2 _returnvalue))
  (bind _bresult (Class|BPIGameModeMP|CanSpawnOneEnemy(Message) (Game|GetGameMode)))
  (if _bresult
    (Variables|Default|SetSpawnPoint _returnvalue_3)
    (while (< (Math|Vector|Distance(Vector) (Variables|Default|GetSpawnPoint) (Transformation|GetActorLocation (Game|GetPlayerController 0))) (Variables|Default|GetMinRange))
      (Variables|Default|SetSpawnPoint _returnvalue_3))
    (AI|SpawnAIFromClass "/Game/AI/BP_Enemy.BP_Enemy_C" 0 _returnvalue_3 "0, 0, 0" false 0)
    (Class|BPIGameModeMP|AddOneEnemy(Message) (Game|GetGameMode))))

(event EventBeginPlay
  (Transformation|SetWorldScale3D (Variables|Default|GetEnemiesSpawnZone) (Variables|Default|GetSpawnScale))
  (Class|BPIGameModeMP|RegisterSpawner(Message) (Game|GetGameMode) self))

(fn ConstructionScript)